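; Endless runner game mode Blueprint that raises the game speed over time.
; BeginPlay starts a looping timer whose event increments CurrentGameSpeed without a cap, writes it to the BG parameter of the PMC_Pinkcity material parameter collection and prints a debug message.
; A separate IncreaseGameSpeed function sets a ScrollSpeed parameter to the incremented speed clamped to MaxGameSpeed, without storing it.
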(event Custom|Increase%20Game%20Speed
  (bind _output_get (Variables|Default|SetCurrentGameSpeed (+ (Variables|Default|GetCurrentGameSpeed) (Variables|Default|GetSpeedIncreaseAmount))))
  (Rendering|Material|SetScalarParameterValue "/Game/Assets/Environments/Background/Materials/PMC_Pinkcity.PMC_Pinkcity" "BG" _output_get :!class /Script/Engine.KismetMaterialLibrary)
  (Development|PrintString "Speed Increasing"))

(event EventBeginPlay
  (Utilities|Time|SetTimerbyEvent (delegate Custom|Increase%20Game%20Speed) (Variables|Default|GetSpeedIncreaseInterval) true))

(fn ConstructionScript)

(fn IncreaseGameSpeed
  (Rendering|Material|SetScalarParameterValue 0 (Variables|Default|GetScroll%20Speed) (Math|Float|Clamp(Float) (+ (Variables|Default|GetCurrentGameSpeed) (Variables|Default|GetSpeedIncreaseAmount)) 0.0 (Variables|Default|GetMaxGameSpeed)) :!class /Script/Engine.KismetMaterialLibrary))