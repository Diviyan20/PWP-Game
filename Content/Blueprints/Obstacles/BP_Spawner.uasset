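; BP_Spawner is an obstacle spawner that repeatedly creates BP_Spikes actors.
; On BeginPlay it starts a looping timer whose interval is randomized once, then each tick of that timer flips a random bool.
; True spawns spikes at the spawner's location; false spawns them at a fixed height with a different rotation and stores the reference in SpikesREF.
; Both branches print the result as debug text.
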(event Custom|Spawn%20Obstacles
  (bind _returnvalue (Transformation|GetActorLocation))
  (bind _output_get (Variables|Default|SetSpawnOnGround (Math|Random|RandomBool)))
  (if _output_get
    (Game|SpawnActorfromClass "/Game/Blueprints/Obstacles/BP_Spikes.BP_Spikes_C" (Math|Transform|MakeTransform (Transformation|GetActorLocation) "0.000000,180.000000,0.000000" "1.000000,1.000000,1.000000") "Undefined" "MultiplyWithRoot" 0 0)
    (Development|PrintString "True")
    (else
      (bind _returnvalue_2 (Game|SpawnActorfromClass "/Game/Blueprints/Obstacles/BP_Spikes.BP_Spikes_C" (Math|Transform|MakeTransform (Math|Vector|MakeVector (.x _returnvalue) (.y _returnvalue) 8.9e+02) "180.000000,0.0,0.0" "1.000000,1.000000,1.000000") "Undefined" "MultiplyWithRoot" 0 0))
      (Variables|Default|SetSpikes%20REF _returnvalue_2)
      (Development|PrintString "False"))))

(event EventBeginPlay
  (Utilities|Time|SetTimerbyEvent (delegate Custom|Spawn%20Obstacles) (Math|Random|RandomFloatinRange 1.0 5.0) true))

(fn ConstructionScript)